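; Enemy turret for a side-scroller that turns to face the player and fires projectiles at them.
; When PawnSensing sees the player character, it snaps the actor's rotation toward them.
; It spawns an EnemyProjectile_BP at the spawn point and launches it with a velocity-change impulse along the cube's forward vector.
; A boolean flag and a short delay throttle the fire rate.
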(event OnSeePawn(PawnSensing)
  (params (Pawn :type Pawn%20Object%20Reference))
  (bind _asside_scroller_character (Utilities|Casting|CastToSideScrollerCharacter Pawn))
  (Utilities|FlowControl|Sequence
    (:then_0
      (Transformation|SetActorRotation (Math|Rotator|FindLookatRotation (Transformation|GetActorLocation) (Transformation|GetActorLocation _asside_scroller_character))))
    (:then_1
      (if (Variables|Default|GetSpawnProjectile)
        (bind _returnvalue (Game|SpawnActorfromClass "/Game/GameContent/Projectiles/EnemyProjectile_BP.EnemyProjectile_BP_C" (Transformation|GetWorldTransform (Variables|Default|GetProjectileSpawnLocation)) "Undefined" 0 0))
        (Physics|AddImpulse (Variables|/Game/GameContent/Projectiles/EnemyProjectile_BP.EnemyProjectile_BP_C|GetProjectile _returnvalue) (* (Math|Vector|GetForwardVector (Variables|Default|GetCube)) (Variables|Default|GetShootAmount)) "None" true)
        (Variables|Default|SetSpawnProjectile false)
        (Utilities|FlowControl|Delay 1.5)
        (Variables|Default|SetSpawnProjectile true)))))

(fn ConstructionScript)