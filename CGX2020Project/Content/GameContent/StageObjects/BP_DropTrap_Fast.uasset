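; Drop trap stage object that releases a burlap bag when a player (I_Player) enters its trigger box and damages players who touch its hurt box.
; A timeline moves the bag and toggles hurt box collision through its Hurt track.
; Impact sound and stone-break particles fire once as the bag nears the bottom, and the trap re-arms when the timeline finishes.
; Older cast-based kill logic remains unconnected.
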(event OnComponentBeginOverlap(TriggerBox)
  (params (OverlappedComponent :type Primitive%20Component%20Object%20Reference) (OtherActor :type Actor%20Object%20Reference) (OtherComp :type Primitive%20Component%20Object%20Reference) (OtherBodyIndex :type Integer) (bFromSweep :type Boolean) (SweepResult :type Hit%20Result%20Structure%20%28by%20ref%29))
  (bind _returnvalue (Transformation|GetActorLocation))
  (if (Utilities|DoesObjectImplementInterface OtherActor "/Game/GameContent/Player/I_Player.I_Player_C")
    (Variables|/Script/Engine.PrimitiveComponent|SetbGenerateOverlapEvents (Variables|Default|GetTrigger%20Box) false)
    (Utilities|FlowControl|DoOnce false :!label _label
      (:Completed
        (Audio|PlaySoundatLocation "/Game/GameContent/Player/Audio/DropTrapRelease.DropTrapRelease" (Transformation|GetActorLocation) "0, 0, 0" 1.0 1.0 0.0 0 0 0)
        (bind (_direction _hurt _newtrack_0) (Timeline|Timeline_0 PlayFromStart)
          (:Update
            (Transformation|SetRelativeLocation (Variables|Default|GetSM_BurlapBag) _newtrack_0 false false)
            (if (< 0.0 _hurt)
              (Collision|SetCollisionEnabled (Variables|Default|GetHurtBox) "NoCollision")
              (else
                (Collision|SetCollisionEnabled (Variables|Default|GetHurtBox) "QueryAndPhysics")))
            (if (< (.Z (Math|Vector|BreakVector _newtrack_0)) 1.0)
              (Utilities|FlowControl|DoOnce false :!label _label_2
                (:Completed
                  (Audio|PlaySoundatLocation "/Game/GameContent/Player/Audio/Impact_Drop_Trap.Impact_Drop_Trap" _returnvalue "0, 0, 0" 1.0 1.0 0.0 0 0 0)
                  (Effects|SpawnEmitteratLocation "/Game/GameContent/IBlade/InfinityBladeEffects/Effects/FX_Breakables/Wall/P_WallBreak_Stone.P_WallBreak_Stone" _returnvalue)))
              (else
                (goto _label_2 Reset))))
          (:Finished
            (Variables|/Script/Engine.PrimitiveComponent|SetbGenerateOverlapEvents (Variables|Default|GetTrigger%20Box) true)
            (goto _label Reset)))))))

(event OnComponentBeginOverlap(SM_BurlapBag)
  (params (OverlappedComponent :type Primitive%20Component%20Object%20Reference) (OtherActor :type Actor%20Object%20Reference) (OtherComp :type Primitive%20Component%20Object%20Reference) (OtherBodyIndex :type Integer) (bFromSweep :type Boolean) (SweepResult :type Hit%20Result%20Structure%20%28by%20ref%29)))

(event OnComponentBeginOverlap(HurtBox)
  (params (OverlappedComponent :type Primitive%20Component%20Object%20Reference) (OtherActor :type Actor%20Object%20Reference) (OtherComp :type Primitive%20Component%20Object%20Reference) (OtherBodyIndex :type Integer) (bFromSweep :type Boolean) (SweepResult :type Hit%20Result%20Structure%20%28by%20ref%29))
  (bind _self self)
  (if (Utilities|DoesObjectImplementInterface OtherActor "/Game/GameContent/Player/I_Player.I_Player_C")
    (Class|IPlayer|DoPlayerDamage(Message) OtherActor 3 (Transformation|GetActorLocation _self) _self)))

(fn ConstructionScript)