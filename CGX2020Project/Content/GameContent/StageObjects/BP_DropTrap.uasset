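; BP_DropTrap is a stage trap that moves a burlap bag when its trigger box is overlapped and kills a Kori that touches its hurt box.
; A timeline drives the bag's relative location and switches the hurt box collision off while its Hurt track is above zero, on otherwise.
; The trigger's overlaps and a DoOnce are re-armed when the timeline finishes, so the trap repeats.
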(event OnComponentBeginOverlap(TriggerBox)
  (params (OverlappedComponent :type Primitive%20Component%20Object%20Reference) (OtherActor :type Actor%20Object%20Reference) (OtherComp :type Primitive%20Component%20Object%20Reference) (OtherBodyIndex :type Integer) (bFromSweep :type Boolean) (SweepResult :type Hit%20Result%20Structure%20%28by%20ref%29))
  (Variables|/Script/Engine.PrimitiveComponent|SetbGenerateOverlapEvents (Variables|Default|GetTrigger%20Box) false)
  (Utilities|FlowControl|DoOnce false :!label _label
    (:Completed
      (bind (_direction _hurt _newtrack_0) (Timeline|Timeline_0 PlayFromStart)
        (:Update
          (Transformation|SetRelativeLocation (Variables|Default|GetSM_BurlapBag) _newtrack_0 false false)
          (if (< 0.0 _hurt)
            (Collision|SetCollisionEnabled (Variables|Default|GetHurtBox) "NoCollision")
            (else
              (Collision|SetCollisionEnabled (Variables|Default|GetHurtBox) "QueryAndPhysics"))))
        (:Finished
          (Variables|/Script/Engine.PrimitiveComponent|SetbGenerateOverlapEvents (Variables|Default|GetTrigger%20Box) true)
          (goto _label Reset))))))

(event OnComponentBeginOverlap(SM_BurlapBag)
  (params (OverlappedComponent :type Primitive%20Component%20Object%20Reference) (OtherActor :type Actor%20Object%20Reference) (OtherComp :type Primitive%20Component%20Object%20Reference) (OtherBodyIndex :type Integer) (bFromSweep :type Boolean) (SweepResult :type Hit%20Result%20Structure%20%28by%20ref%29)))

(event OnComponentBeginOverlap(HurtBox)
  (params (OverlappedComponent :type Primitive%20Component%20Object%20Reference) (OtherActor :type Actor%20Object%20Reference) (OtherComp :type Primitive%20Component%20Object%20Reference) (OtherBodyIndex :type Integer) (bFromSweep :type Boolean) (SweepResult :type Hit%20Result%20Structure%20%28by%20ref%29))
  (bind _askori (Utilities|Casting|CastToKori OtherActor))
  (Development|PrintString "IT HURT!@!@!@#!@#")
  (Default|KillKori _askori))

(fn ConstructionScript)