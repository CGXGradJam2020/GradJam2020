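; BP_SlammableObject is a stage object that gets knocked away from the player when broken.
; The construction script sets the body mesh from the first entry of its object list.
; DoBreak turns on physics, then sets the mesh's velocity along the direction away from the player pawn, using only Y and Z with separate horizontal and vertical multipliers.
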(event EventBeginPlay)

(event Collision|EventActorBeginOverlap
  (params (OtherActor :type Actor%20Object%20Reference)))

(event EventTick
  (params (DeltaSeconds :type Float%20%28single-precision%29)))

(event EventDoBreak
  (bind _returnvalue (Game|Player|GetPlayerPawn 0))
  (bind _bodymesh (Variables|Default|GetBodyMesh))
  (bind _bodymesh_2 (Variables|Default|GetBodyMesh))
  (bind _returnvalue_2 (Transformation|GetActorLocation _returnvalue))
  (bind _returnvalue_3 (Transformation|GetWorldLocation _bodymesh))
  (bind _returnvalue_4 (- _returnvalue_3 _returnvalue_2))
  (bind _returnvalue_5 (Math|Vector|Normalize _returnvalue_4))
  (Physics|SetSimulatePhysics _bodymesh_2 true)
  (Physics|SetPhysicsLinearVelocity _bodymesh_2 (Math|Vector|MakeVector 0.0 (* (.y _returnvalue_5) (Variables|Default|GetHorizontalImpulseMult)) (* (.z _returnvalue_5) (Variables|Default|GetVerticalImpulseMult))) false "None"))

(fn ConstructionScript
  (Components|StaticMesh|SetStaticMesh (Variables|Default|GetBodyMesh) (Utilities|Array|Get(acopy) (Variables|Default|GetObjectsList))))